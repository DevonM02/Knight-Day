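; Moving platform that travels along the spline of a SplinePathBP1 actor found in the level at BeginPlay.
; A timeline drives its MoveTrack alpha across the spline's length, setting the actor's world location and rotation from the spline each update.
; The timeline play rate is the inverse of TimeToCompleteInSeconds, so that variable controls the travel time.
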(event Custom|Move%20Object
  (bind _spline_ref1 (Variables|Default|GetSpline%20REF1))
  (bind _spline (Variables|/Game/Blueprints/SplinePathBP1.SplinePathBP1_C|GetSpline _spline_ref1))
  (Components|Timeline|SetPlayRate (Variables|Default|GetMove%20Object_T) (/ 1.0 (Variables|Default|GetTime%20To%20Complete%20%28in%20Seconds%29)))
  (bind _move_track (Timeline|Move%20Object_T Play)
    (:Update
      (Transformation|SetActorTransform (Math|Transform|MakeTransform (Spline|GetLocationatDistanceAlongSpline _spline (Math|Float|Lerp 0.0 (Spline|GetSplineLength (Variables|/Game/Blueprints/SplinePathBP1.SplinePathBP1_C|GetSpline (Variables|Default|GetSpline%20REF1))) _move_track) "World") (Spline|GetRotationatDistanceAlongSpline _spline (Math|Float|Lerp 0.0 (Spline|GetSplineLength (Variables|/Game/Blueprints/SplinePathBP1.SplinePathBP1_C|GetSpline (Variables|Default|GetSpline%20REF1))) _move_track) "World") "1,1,1")))))

(event EventBeginPlay
  (bind _returnvalue (Actor|GetActorOfClass "/Game/Blueprints/SplinePathBP1.SplinePathBP1_C"))
  (Variables|Default|SetSpline%20REF1 _returnvalue)
  (CallFunction|MoveObject))

(fn ConstructionScript)