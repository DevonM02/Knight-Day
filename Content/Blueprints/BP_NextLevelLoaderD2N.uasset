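; Interactable level-transition actor that sends the player to another level at a chosen spawn location.
; Interact stores SpawnLocation on MyGameInstance and calls its smooth level load with LevelToLoad, disabling player input before and re-enabling it immediately after the call.
; Sphere overlaps show and hide a prompt widget, while RemovePrompts alternately hides and restores it in game through a FlipFlop.
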(event OnComponentBeginOverlap(Sphere)
  (params (OverlappedComponent :type Primitive%20Component%20Object%20Reference) (OtherActor :type Actor%20Object%20Reference) (OtherComp :type Primitive%20Component%20Object%20Reference) (OtherBodyIndex :type Integer) (bFromSweep :type Boolean) (SweepResult :type Hit%20Result%20Structure%20%28by%20ref%29))
  (Rendering|SetVisibility (Variables|Default|GetWidget) true false))

(event OnComponentEndOverlap(Sphere)
  (params (OverlappedComponent :type Primitive%20Component%20Object%20Reference) (OtherActor :type Actor%20Object%20Reference) (OtherComp :type Primitive%20Component%20Object%20Reference) (OtherBodyIndex :type Integer))
  (Rendering|SetVisibility (Variables|Default|GetWidget) false false))

(event EventInteract
  (bind _returnvalue (Game|GetPlayerCharacter 0))
  (bind _returnvalue_2 (Game|GetPlayerController 0))
  (Input|DisableInput _returnvalue _returnvalue_2)
  (bind _asmy_game_instance (Utilities|Casting|CastToMyGameInstance (Game|GetGameInstance)))
  (Variables|/Game/MyGameInstance.MyGameInstance_C|SetSpawn_Loc _asmy_game_instance (Variables|Default|GetSpawn_Location))
  (Default|EventSmoothLoadLevel _asmy_game_instance (Variables|Default|GetLevel%20To%20Load))
  (Input|EnableInput _returnvalue _returnvalue_2))

(event EventRemovePrompts
  (bind _widget (Variables|Default|GetWidget))
  (Utilities|FlowControl|FlipFlop
    (:A
      (Development|SetHiddeninGame _widget true false))
    (:B
      (Development|SetHiddeninGame _widget false false))))

(fn ConstructionScript)